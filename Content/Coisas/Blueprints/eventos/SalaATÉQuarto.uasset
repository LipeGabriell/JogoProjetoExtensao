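; Trigger event actor that moves the player between rooms, named for living room to bedroom but prompting "Banheiro" (bathroom).
; When PersonagemFase1 overlaps it, it enables input, shows a TextoInteract widget and opens a Gate.
; Pressing E passes the Gate, removes the prompt and teleports the pawn to a hard-coded location and rotation.
; Leaving the overlap disables input, removes the prompt and closes the Gate.
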(event `self.ReceiveActorBeginOverlap`
  (params (OtherActor :type "Actor Object Reference"))
  (bind _returnvalue (`GameplayStatics.GetPlayerPawn` 0))
  ;[1 0.9405 0.1679] Texto cima
  (cast `/Game/Coisas/Blueprints/personagemCOISAS/PersonagemFase1` OtherActor)
  (`self.EnableInput` (`GameplayStatics.GetPlayerController` 0))
  (bind _returnvalue_2 (`|CreateWidget` "/Game/Coisas/Blueprints/eventos/UI/textoInteract.textoInteract_C" null "Banheiro"))
  (`UserWidget.AddToViewport` _returnvalue_2 0)
  (goto _label :!via `Open`))

(event `self.ReceiveActorEndOverlap`
  (params (OtherActor :type "Actor Object Reference"))
  (bind _returnvalue (`GameplayStatics.GetPlayerPawn` 0))
  ;[1 0.9405 0.1679] Texto cima
  (cast `/Game/Coisas/Blueprints/personagemCOISAS/PersonagemFase1` OtherActor)
  (`self.DisableInput` (`GameplayStatics.GetPlayerController` 0))
  (`Widget.RemoveFromParent` null)
  (`Widget.RemoveFromParent` (stale `self.ReceiveActorBeginOverlap` _returnvalue_2))
  (goto _label :!via `Close`))

(event `Key|E`
  (params (Key :type "Key Structure"))
  (bind _returnvalue (`GameplayStatics.GetPlayerPawn` 0))
  ;[1 0.9405 0.1679] Texto cima
  (:`Pressed`
    (`/Engine/EditorBlueprintResources/StandardMacros.Gate` true :!label _label
      (:`Exit`
        (`Widget.RemoveFromParent` (stale `self.ReceiveActorBeginOverlap` _returnvalue_2))
        (`Widget.RemoveFromParent` null)
        (`self.K2_SetActorTransform` _returnvalue (`KismetMathLibrary.Conv_VectorToTransform` (163.0 870.0 230.0)) false false)
        (`self.K2_SetActorRotation` _returnvalue (struct :`Yaw` 270.0) false)))))

(fn `UserConstructionScript`)