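; Interactable ointment (pomada) pickup that explains the item's use on first-degree burns and lets the Fase 1 character collect it.
; Overlap by PersonagemFase1 enables input and shows a title widget and an info widget; leaving disables input and removes both.
; A Gate limits the E key to the overlap window.
; Pickup destroys the collision and linked actor, lowers this actor, sets PomadaPEGOU and plays a click sound.
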(event `self.ReceiveActorBeginOverlap`
  (params (OtherActor :type "Actor Object Reference"))
  ;[1 0.9405 0.1679] Texto cima
  (cast `/Game/Coisas/Blueprints/personagemCOISAS/PersonagemFase1` OtherActor)
  (`KismetSystemLibrary.PrintString` "entrou")
  (`self.EnableInput` (`GameplayStatics.GetPlayerController` 0))
  (bind _returnvalue (`|CreateWidget` "/Game/Coisas/Blueprints/eventos/textoCima.textoCima_C" null "  "))
  (bind _returnvalue_2 (`|CreateWidget` "/Game/Coisas/Blueprints/eventos/textoInteract.textoInteract_C" null "Pode ser aplicada em queimaduras 1° grau com sintomas de dor, vermelhidão e/ou inchaço. As pomadas aliviam e podem ser usadas sem prescrição médica. Caso seu uso não resolva procure um médico."))
  (set `/Game/Coisas/Blueprints/eventos/textoCima.Texto Cima` (`self.texto do interact`) _returnvalue)
  (`UserWidget.AddToViewport` _returnvalue 0)
  (`UserWidget.AddToViewport` null 0)
  (`UserWidget.AddToViewport` _returnvalue_2 0)
  (goto _label :!via `Open`))

(event `self.ReceiveActorEndOverlap`
  (params (OtherActor :type "Actor Object Reference"))
  ;[1 0.9405 0.1679] Texto cima
  (cast `/Game/Coisas/Blueprints/personagemCOISAS/PersonagemFase1` OtherActor)
  (`KismetSystemLibrary.PrintString` "saiu")
  (`self.DisableInput` (`GameplayStatics.GetPlayerController` 0))
  (`Widget.RemoveFromParent` (stale `self.ReceiveActorBeginOverlap` _returnvalue))
  (`Widget.RemoveFromParent` null)
  (`Widget.RemoveFromParent` (stale `self.ReceiveActorBeginOverlap` _returnvalue_2))
  (goto _label :!via `Close`))

(event `Key|E`
  (params (Key :type "Key Structure"))
  ;[1 0.9405 0.1679] Texto cima
  (:`Pressed`
    (`/Engine/EditorBlueprintResources/StandardMacros.Gate` true :!label _label
      (:`Exit`
        (`ActorComponent.K2_DestroyComponent` (`self.CollisionComponent`))
        (`ActorComponent.K2_DestroyComponent` (`self.TriggerBox_3`))
        (`Widget.RemoveFromParent` (stale `self.ReceiveActorBeginOverlap` _returnvalue))
        (`Widget.RemoveFromParent` null)
        (`self.K2_SetActorRelativeLocation` (0.0 0.0 -100.0))
        (`self.K2_DestroyActor` (`self.Ator`))
        (set `self.Pomada PEGOU` true)
        (`GameplayStatics.PlaySound2D` "/Game/Coisas/mapas/menu/somClica.somClica" 1.0 1.0 0.0 null null)))))

(fn `UserConstructionScript`)