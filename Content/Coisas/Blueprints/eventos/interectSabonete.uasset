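; Interaction trigger for the neutral soap ("sabonete") pickup, which shows Portuguese first-aid advice on treating burns.
; When PersonagemFase1 overlaps it, it enables input, adds two text widgets and opens a Gate; leaving reverses this.
; Pressing E through the open Gate destroys the collision and linked item actor, removes the top widget, lowers itself, sets SabonetePEGOU and plays a click sound.
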(event `self.ReceiveActorBeginOverlap`
  (params (OtherActor :type "Actor Object Reference"))
  ;[1 0.9405 0.1679] Texto cima
  (cast `/Game/Coisas/Blueprints/personagemCOISAS/PersonagemFase1` OtherActor)
  (`KismetSystemLibrary.PrintString` "entrou")
  (`self.EnableInput` (`GameplayStatics.GetPlayerController` 0))
  (bind _returnvalue (`|CreateWidget` "/Game/Coisas/Blueprints/eventos/textoCima.textoCima_C" null "  "))
  (bind _returnvalue_2 (`|CreateWidget` "/Game/Coisas/Blueprints/eventos/textoInteract.textoInteract_C" null "Ao usar o sabonete neutro em queimaduras de 1° grau é preciso antes lavar com água fria por 5 minutos para esfriar a pele e limpa-la de microrganismos. Após a limpeza é ideal fazer compressa frias  e depois hidratar a pele. \nEm queimaduras de 2° grau também irá lavar o rosto e depois passar o sabonete, porém, agora será por 10 minutos. Tente não pocar as bolhas na hora de passar o sabonete e não mexer nelas. Se for preciso procure um médico para fazer o tratamento correto das queimaduras. \n"))
  (set `/Game/Coisas/Blueprints/eventos/textoCima.Texto Cima` (`self.texto do interact`) _returnvalue)
  (`UserWidget.AddToViewport` _returnvalue 0)
  (`UserWidget.AddToViewport` null 0)
  (`UserWidget.AddToViewport` _returnvalue_2 0)
  (goto _label :!via `Open`))

(event `self.ReceiveActorEndOverlap`
  (params (OtherActor :type "Actor Object Reference"))
  ;[1 0.9405 0.1679] Texto cima
  (cast `/Game/Coisas/Blueprints/personagemCOISAS/PersonagemFase1` OtherActor)
  (`KismetSystemLibrary.PrintString` "saiu")
  (`self.DisableInput` (`GameplayStatics.GetPlayerController` 0))
  (`Widget.RemoveFromParent` (stale `self.ReceiveActorBeginOverlap` _returnvalue))
  (`Widget.RemoveFromParent` null)
  (`Widget.RemoveFromParent` (stale `self.ReceiveActorBeginOverlap` _returnvalue_2))
  (goto _label :!via `Close`))

(event `Key|E`
  (params (Key :type "Key Structure"))
  ;[1 0.9405 0.1679] Texto cima
  (:`Pressed`
    (`/Engine/EditorBlueprintResources/StandardMacros.Gate` true :!label _label
      (:`Exit`
        (`ActorComponent.K2_DestroyComponent` (`self.CollisionComponent`))
        (`ActorComponent.K2_DestroyComponent` (`self.TriggerBox_3`))
        (`Widget.RemoveFromParent` (stale `self.ReceiveActorBeginOverlap` _returnvalue))
        (`self.K2_SetActorRelativeLocation` (0.0 0.0 -100.0))
        (`self.K2_DestroyActor` (`self.Ator`))
        (set `self.Sabonete PEGOU` true)
        (`GameplayStatics.PlaySound2D` "/Game/Coisas/mapas/menu/somClica.somClica" 1.0 1.0 0.0 null null)))))

(fn `UserConstructionScript`)