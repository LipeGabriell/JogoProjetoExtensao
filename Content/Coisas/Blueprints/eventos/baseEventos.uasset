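; Interaction trigger, likely a base for events, where the phase 1 character presses E to remove the trigger and a referenced actor, Ator.
; Overlap by PersonagemFase1 enables input, shows a TextoCima widget with TextoDoInteract and a TextoInteract widget, and opens a Gate.
; Pressing E passes through the Gate to destroy collision components, widgets and both actors.
; Leaving the overlap disables input, removes the widgets and closes the Gate.
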(event `self.ReceiveActorBeginOverlap`
  (params (OtherActor :type "Actor Object Reference"))
  ;[1 0.9405 0.1679] Texto cima
  (cast `/Game/Coisas/Blueprints/personagemCOISAS/PersonagemFase1` OtherActor)
  (`self.EnableInput` (`GameplayStatics.GetPlayerController` 0))
  (bind _returnvalue (`|CreateWidget` "/Game/Coisas/Blueprints/eventos/UI/textoCima.textoCima_C" null "  "))
  (set `/Game/Coisas/Blueprints/eventos/UI/textoCima.Texto Cima` (`self.texto do interact`) _returnvalue)
  (bind _returnvalue_2 (`|CreateWidget` "/Game/Coisas/Blueprints/eventos/UI/textoInteract.textoInteract_C"))
  (`UserWidget.AddToViewport` _returnvalue 0)
  (`UserWidget.AddToViewport` _returnvalue_2 0)
  (goto _label :!via `Open`))

(event `self.ReceiveActorEndOverlap`
  (params (OtherActor :type "Actor Object Reference"))
  ;[1 0.9405 0.1679] Texto cima
  (cast `/Game/Coisas/Blueprints/personagemCOISAS/PersonagemFase1` OtherActor)
  (`self.DisableInput` (`GameplayStatics.GetPlayerController` 0))
  (`Widget.RemoveFromParent` (stale `self.ReceiveActorBeginOverlap` _returnvalue))
  (`Widget.RemoveFromParent` (stale `self.ReceiveActorBeginOverlap` _returnvalue_2))
  (goto _label :!via `Close`))

(event `Key|E`
  (params (Key :type "Key Structure"))
  ;[1 0.9405 0.1679] Texto cima
  (:`Pressed`
    (`/Engine/EditorBlueprintResources/StandardMacros.Gate` true :!label _label
      (:`Exit`
        (`ActorComponent.K2_DestroyComponent` (`self.CollisionComponent`))
        (`ActorComponent.K2_DestroyComponent` (`self.TriggerBox_3`))
        (`Widget.RemoveFromParent` (stale `self.ReceiveActorBeginOverlap` _returnvalue))
        (`Widget.RemoveFromParent` (stale `self.ReceiveActorBeginOverlap` _returnvalue_2))
        (`self.K2_DestroyActor`)
        (`self.K2_DestroyActor` (`self.Ator`))))))

(fn `UserConstructionScript`)