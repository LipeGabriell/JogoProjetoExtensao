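; Gauze pickup trigger that shows the Fase 1 character (PersonagemFase1) a prompt and a Portuguese first-aid text about gauze.
; Overlap enables input and adds both widgets, while leaving disables input and removes them.
; A Gate limits the E key to the overlap: pressing it destroys the trigger components and gauze actor, removes the top prompt, sets GazePEGOU and plays a click sound.
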(event `self.ReceiveActorBeginOverlap`
  (params (OtherActor :type "Actor Object Reference"))
  ;[1 0.9405 0.1679] Texto cima
  (cast `/Game/Coisas/Blueprints/personagemCOISAS/PersonagemFase1` OtherActor)
  (`self.EnableInput` (`GameplayStatics.GetPlayerController` 0))
  (bind _returnvalue (`|CreateWidget` "/Game/Coisas/Blueprints/eventos/UI/textoCima.textoCima_C" null "TEXTO GAZE AQUI"))
  (bind _returnvalue_2 (`|CreateWidget` "/Game/Coisas/Blueprints/eventos/UI/textoInteract.textoInteract_C" null "A gaze é uma compressa que serve como um curativo contra as feridas. A gaze pode ser utilizada em primeiros socorros para ferimentos simples e mais graves. Após utilizar a gaze, a ferida deve ser limpa, assim como a mão de quem fez o uso. A gaze deve ser trocada após utilizada."))
  (set `/Game/Coisas/Blueprints/eventos/UI/textoCima.Texto Cima` (`self.texto do interact`) _returnvalue)
  (`UserWidget.AddToViewport` _returnvalue 0)
  (`UserWidget.AddToViewport` null 0)
  (`UserWidget.AddToViewport` _returnvalue_2 0)
  (goto _label :!via `Open`))

(event `self.ReceiveActorEndOverlap`
  (params (OtherActor :type "Actor Object Reference"))
  ;[1 0.9405 0.1679] Texto cima
  (cast `/Game/Coisas/Blueprints/personagemCOISAS/PersonagemFase1` OtherActor)
  (`self.DisableInput` (`GameplayStatics.GetPlayerController` 0))
  (`Widget.RemoveFromParent` (stale `self.ReceiveActorBeginOverlap` _returnvalue))
  (`Widget.RemoveFromParent` null)
  (`Widget.RemoveFromParent` (stale `self.ReceiveActorBeginOverlap` _returnvalue_2))
  (goto _label :!via `Close`))

(event `Key|E`
  (params (Key :type "Key Structure"))
  ;[1 0.9405 0.1679] Texto cima
  (:`Pressed`
    (`/Engine/EditorBlueprintResources/StandardMacros.Gate` true :!label _label
      (:`Exit`
        (`ActorComponent.K2_DestroyComponent` (`self.CollisionComponent`))
        (`ActorComponent.K2_DestroyComponent` (`self.TriggerBox_3`))
        (`Widget.RemoveFromParent` (stale `self.ReceiveActorBeginOverlap` _returnvalue))
        (`self.K2_DestroyActor` (`self.ator gaze`))
        (set `self.Gaze PEGOU` true)
        (`GameplayStatics.PlaySound2D` "/Game/Coisas/mapas/menu/somClica.somClica" 1.0 1.0 0.0 null null)))))

(fn `UserConstructionScript`)