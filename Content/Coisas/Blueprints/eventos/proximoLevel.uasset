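; End-of-level trigger actor where the Fase 1 character delivers with E to finish the level.
; Overlap enables input, shows a Portuguese interact prompt and opens a Gate; leaving reverses all three.
; E fires through the Gate, destroying the trigger components and the actor, swapping in the final text widget and setting FinalTrue.
; A five-second Delay, placed after DestroyActor, precedes loading the menu level.
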(event `self.ReceiveActorBeginOverlap`
  (params (OtherActor :type "Actor Object Reference"))
  (bind _returnvalue (`GameplayStatics.GetPlayerController` 0))
  ;[1 0.9405 0.1679] Texto cima
  (cast `/Game/Coisas/Blueprints/personagemCOISAS/PersonagemFase1` OtherActor)
  (`KismetSystemLibrary.PrintString` "entrou")
  (`self.EnableInput` _returnvalue)
  (bind _returnvalue_2 (`|CreateWidget` "/Game/Coisas/Blueprints/eventos/textoInteract.textoInteract_C" _returnvalue "Aperte \"E\" para entregar"))
  (`UserWidget.AddToViewport` _returnvalue_2 0)
  (goto _label :!via `Open`))

(event `self.ReceiveActorEndOverlap`
  (params (OtherActor :type "Actor Object Reference"))
  (bind _returnvalue (`GameplayStatics.GetPlayerController` 0))
  ;[1 0.9405 0.1679] Texto cima
  (cast `/Game/Coisas/Blueprints/personagemCOISAS/PersonagemFase1` OtherActor)
  (`KismetSystemLibrary.PrintString` "saiu")
  (`self.DisableInput` _returnvalue)
  (`Widget.RemoveFromParent` (stale `self.ReceiveActorBeginOverlap` _returnvalue_2))
  (goto _label :!via `Close`))

(event `Key|E`
  (params (Key :type "Key Structure"))
  ;[1 0.9405 0.1679] Texto cima
  (:`Pressed`
    (`/Engine/EditorBlueprintResources/StandardMacros.Gate` true :!label _label
      (:`Exit`
        (`ActorComponent.K2_DestroyComponent` (`self.CollisionComponent`))
        (`ActorComponent.K2_DestroyComponent` (`self.TriggerBox_3`))
        (`self.K2_DestroyActor`)
        (`Widget.RemoveFromParent` (stale `self.ReceiveActorBeginOverlap` _returnvalue_2))
        (bind _returnvalue (`|CreateWidget` "/Game/Coisas/Blueprints/eventos/textoFINAL.textoFINAL_C" (`GameplayStatics.GetPlayerController` 0)))
        (`UserWidget.AddToViewport` _returnvalue 0)
        (set `self.finalTrue` true)
        (`KismetSystemLibrary.Delay` 5.0)
        (`GameplayStatics.OpenLevel` "menu")))))

(fn `UserConstructionScript`)